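; VPTK_TrackedActorComponent is a virtual production toolkit component that lets its owning actor follow an assigned tracker head.
; On BeginPlay it registers the owner in the player state's TrackedActors list for discovery.
; AssignToTracker stores the head and activates tracking, then Tick copies its transform to the owner.
; Optional noise reduction routes through helpers meant to round location and rotation, though their nodes appear unconnected.
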(event `self.ReceiveBeginPlay`
  ;[1 1 1] Register this Tracked Actor so the volume can discover it
  (bind _asvptk_player_state_base (cast `/Game/VPToolKit/BluePrint/VPTK_PlayerStateBAse` (`Controller.PlayerState` (`GameplayStatics.GetPlayerController` 0))))
  (`KismetArrayLibrary.Array_AddUnique` (`/Game/VPToolKit/BluePrint/VPTK_PlayerStateBAse.TrackedActors` _asvptk_player_state_base) (`self.GetOwner`)))

(event `self.ReceiveTick`
  (params (DeltaSeconds :type "Float (single-precision)"))
  (bind _returnvalue (`self.GetOwner`))
  (bind _assignedtrackerhead (`self.assignedTrackerHead`))
  (bind _returnvalue_2 (`Actor.GetTransform` _assignedtrackerhead))
  ;[1 1 1] Update the world transform from the tracker head
  (if (`self.TackerActive`)
    (if (`KismetSystemLibrary.IsValid` _assignedtrackerhead)
      (if (`self.Enable Noise Reduction`)
        (`Actor.K2_SetActorTransform` _returnvalue (`self.ReduceTransformNoise` _returnvalue_2) false false)
        (else
          (`Actor.K2_SetActorTransform` _returnvalue _returnvalue_2 false false))))))

(fn `AssignToTracker`
  (params (trackerID :type Integer) (TrackerHead :type "Actor Object Reference"))
  (set `self.assignedTrackerID` trackerID)
  (set `self.assignedTrackerHead` TrackerHead)
  (set `self.TackerActive` true))