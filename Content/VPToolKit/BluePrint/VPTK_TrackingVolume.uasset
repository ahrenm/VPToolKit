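; VPTK tracking volume actor: the virtual production controller that maps tracked devices onto registered actors and sets up the HUD.
; On BeginPlay it scans device IDs, builds a name-keyed table from self-registered TrackedActorComponents and assigns desired trackers, switching the view to camera actors.
; Tick drives attached proxy actors from device poses, with child actors carrying each component's offset.
; Input actions toggle the HUD, control four sequences and trigger four interface-based actor actions.
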(event `self.ReceiveBeginPlay`
  (bind _returnvalue (`GameplayStatics.GetPlayerController` 0))
  (bind _trackedentities (`self.TrackedEntities`))
  (bind _trackedactors (`/Game/VPToolKit/BluePrint/VPTK_PlayerStateBAse.TrackedActors` (`self.PlayerStateRef`)))
  ;[0.57 0.6196 1] BeginPlay
  ;[1 1 1] Setup the base environment
  (`self.WriteVPLog` "Starting VPTK Controller....")
  (bind _asvptk_player_state_base (cast `/Game/VPToolKit/BluePrint/VPTK_PlayerStateBAse` (`Controller.PlayerState` (`GameplayStatics.GetPlayerController` 0)))
    (:`then`
      (bind _output_get (set `self.PlayerStateRef` _asvptk_player_state_base))
      (set `/Game/VPToolKit/BluePrint/VPTK_PlayerStateBAse.TrackingVolume` self _output_get)
      (`self.WriteVPLog` "Wiating for Tracked Actors to register with volme")
      (`KismetSystemLibrary.Delay` 1.0) ; Delay here to allow the components to sign in
      ;[1 1 1] Search for trackers
      (`self.WriteVPLog` "Scanning for trackers...")
      (for _array_element (`SteamVRFunctionLibrary.GetValidTrackedDeviceIds` "Controller")
        (`KismetArrayLibrary.Array_Add` (`self.AvaliableTrackingIds`) _array_element)
        (`self.WriteVPLog` (`KismetStringLibrary.BuildString_Int` "Found controller at tracking id : " "" _array_element)))
      (for _array_element_2 (`SteamVRFunctionLibrary.GetValidTrackedDeviceIds` "Other")
        (`KismetArrayLibrary.Array_Add` (`self.AvaliableTrackingIds`) _array_element_2)
        (`self.WriteVPLog` (`KismetStringLibrary.BuildString_Int` "Found other device at tracking id : " "" _array_element_2)))
      ;[1 1 1] Create Tracking Dataset
      (`self.WriteVPLog` (`KismetStringLibrary.BuildString_Int` "" "Building Actor tracking table with " (`KismetArrayLibrary.Array_Length` _trackedactors) " Actors auto registered"))
      (for _array_element_3 _trackedactors
        (bind _tracked_actor_component (`self.GetTrackedActorComponent` _array_element_3))
        (bind _name (`/Game/VPToolKit/BluePrint/VPTK_TrackedActorComponent.Name` _tracked_actor_component))
        (if (`KismetStringLibrary.IsEmpty` _name)
          (bind _returnvalue_2 (`ActorComponent.GetOwner` _tracked_actor_component))
          ;;[1 0.1471 0.1332] Error handling
          (`self.WriteVPLog` (`KismetStringLibrary.BuildString_Object` "" "ERROR: TrackedActorComponent attached to :" _returnvalue_2 " requires a vaild name"))
          (elif (`BlueprintMapLibrary.Map_Contains` _trackedentities _name)
            (`self.WriteVPLog` (`KismetStringLibrary.BuildString_Object` "" "ERROR: TrackedActorComponent attached to " _returnvalue_2 "does not have a unique name"))
            (else
              (bind _returnvalue_3 (`|SpawnActorFromClass` "/Game/VPToolKit/BluePrint/EmptyActor.EmptyActor_C" (`KismetMathLibrary.MakeTransform` (0.0 0.0 0.0)) "Undefined" "OverrideRootScale" null null)) ; Tracker Actual Ref
              (`self.K2_AttachToActor` _returnvalue_3 self "None" "KeepRelative" "KeepRelative" "KeepRelative" false) ; Attach to tracking volume
              (bind (_offset_location _offset_rotation _offset_scale) (`KismetMathLibrary.BreakTransform` (`/Game/VPToolKit/BluePrint/VPTK_TrackedActorComponent.Offset` _tracked_actor_component)))
              (bind _returnvalue_4 (`|SpawnActorFromClass` "/Game/VPToolKit/BluePrint/EmptyActor.EmptyActor_C" (`KismetMathLibrary.MakeTransform` (0.0 0.0 0.0) _offset_rotation _offset_scale) "Undefined" "OverrideRootScale" null null)) ; Head Object
              (`self.K2_AttachToActor` _returnvalue_4 _returnvalue_3 "None" "KeepRelative" "KeepRelative" "KeepRelative" true)
              (`SceneComponent.K2_AddWorldTransform` (`Actor.RootComponent` _returnvalue_4) (`KismetMathLibrary.MakeTransform` _offset_location (struct)) false false)
              (`BlueprintMapLibrary.Map_Add` _trackedentities _name (make `/Game/VPToolKit/BluePrint/VPTK_TrackedEntity` -1 _returnvalue_3 _returnvalue_4 _tracked_actor_component))))))
      ;[1 1 1] Try to assign to desired IDs
      (bind _values (`BlueprintMapLibrary.Map_Values` (`self.TrackedEntities`)))
      (for _array_element_4 _values
        (`self.Assign Actor to Tracker` (`/Game/VPToolKit/BluePrint/VPTK_TrackedActorComponent.Name` (`.TrackedActorComponent_14_D43A9CD84B528C7316EC1EBA682D77DA` (break `/Game/VPToolKit/BluePrint/VPTK_TrackedEntity` _array_element_4))) (`/Game/VPToolKit/BluePrint/VPTK_TrackedActorComponent.DesiredTrackerID` (`.TrackedActorComponent_14_D43A9CD84B528C7316EC1EBA682D77DA` (break `/Game/VPToolKit/BluePrint/VPTK_TrackedEntity` _array_element_4)))))
      ;[1 1 1] Initalise the HUD
      (bind _asvptk_hud (cast `/Game/VPToolKit/BluePrint/UI/VPTK_HUD` (`PlayerController.GetHUD` _returnvalue))
        (:`then`
          (bind _output_get_2 (set `self.HUD` _asvptk_hud))
          (`/Game/VPToolKit/BluePrint/UI/VPTK_HUD.InitaliseHUD` _output_get_2 self)
          (`self.EnableInput` _returnvalue)
          (if (not (`self.MenuEnabledOn Start`))
            (`/Game/VPToolKit/BluePrint/UI/VPTK_HUD.ToggleVisability` (`self.HUD`)))
          (`self.WriteVPLog` "Startup complete"))
        (:`CastFailed`
          (`KismetSystemLibrary.PrintString` "ERROR VPTK CAST TO HUD FAILED" true true (struct :`R` 1.0 :`B` 0.110131 :`A` 1.0)))))
    (:`CastFailed`
      (`KismetSystemLibrary.PrintString` "ERROR! VPTK Failed to find PlayerState!"))))

(event `self.ReceiveTick`
  (params (DeltaSeconds :type "Float (single-precision)"))
  ;[1 1 1] On Tick update the tracker reference actors with the new transforms
  (if (`self.Tracking Active`)
    (bind _values (`BlueprintMapLibrary.Map_Values` (`self.TrackedEntities`)))
    (for _array_element _values
      (if (> (break `/Game/VPToolKit/BluePrint/VPTK_TrackedEntity` _array_element) 0)
        (bind (_outposition _outorientation _returnvalue) (`SteamVRFunctionLibrary.GetTrackedDevicePositionAndOrientation` (break `/Game/VPToolKit/BluePrint/VPTK_TrackedEntity` _array_element)))
        (if _returnvalue
          (`self.K2_SetActorRelativeTransform` (`.TrackerVirtualObject_8_3B16C4C141F8D81EF7647BA531DB1EB0` (break `/Game/VPToolKit/BluePrint/VPTK_TrackedEntity` _array_element)) (`KismetMathLibrary.MakeTransform` _outposition _outorientation) false false))))))

(event `InputAction|VP_HUD_Toggle`
  (params (Key :type "Key Structure"))
  ;[1 1 1] Toggle Menu Visability
  (:`Pressed`
    (`/Game/VPToolKit/BluePrint/UI/VPTK_HUD.ToggleVisability` (`self.HUD`))))

(event `InputAction|VP_Triggerable_1`
  (params (Key :type "Key Structure"))
  (bind _sequenceplayer (`LevelSequenceActor.SequencePlayer` (`self.Sequence1`)))
  ;[1 1 1] Sequence 1 Control
  (:`Pressed`
    (if (`MovieSceneSequencePlayer.IsPlaying` _sequenceplayer)
      (`MovieSceneSequencePlayer.Pause` _sequenceplayer)
      (else
        (`MovieSceneSequencePlayer.Play` _sequenceplayer)))))

(event `InputAction|VP_Triggerable_1_Stop`
  (params (Key :type "Key Structure"))
  ;[1 1 1] Sequence 1 Control
  (:`Pressed`
    (`MovieSceneSequencePlayer.Stop` (`LevelSequenceActor.SequencePlayer` (`self.Sequence1`)))))

(event `InputAction|VP_Triggerable_2`
  (params (Key :type "Key Structure"))
  (bind _sequenceplayer (`LevelSequenceActor.SequencePlayer` (`self.Sequence2`)))
  ;[1 1 1] Sequence 2 Control
  (:`Pressed`
    (if (`MovieSceneSequencePlayer.IsPlaying` _sequenceplayer)
      (`MovieSceneSequencePlayer.Pause` _sequenceplayer)
      (else
        (`MovieSceneSequencePlayer.Play` _sequenceplayer)))))

(event `InputAction|VP_Triggerable_2_Stop`
  (params (Key :type "Key Structure"))
  ;[1 1 1] Sequence 2 Control
  (:`Pressed`
    (`MovieSceneSequencePlayer.Stop` (`LevelSequenceActor.SequencePlayer` (`self.Sequence2`)))))

(event `InputAction|VP_Triggerable_3`
  (params (Key :type "Key Structure"))
  (bind _sequenceplayer (`LevelSequenceActor.SequencePlayer` (`self.Sequence3`)))
  ;[1 1 1] Sequence 3 Control
  (:`Pressed`
    (if (`MovieSceneSequencePlayer.IsPlaying` _sequenceplayer)
      (`MovieSceneSequencePlayer.Pause` _sequenceplayer)
      (else
        (`MovieSceneSequencePlayer.Play` _sequenceplayer)))))

(event `InputAction|VP_Triggerable_3_Stop`
  (params (Key :type "Key Structure"))
  ;[1 1 1] Sequence 3 Control
  (:`Pressed`
    (`MovieSceneSequencePlayer.Stop` (`LevelSequenceActor.SequencePlayer` (`self.Sequence3`)))))

(event `InputAction|VP_Triggerable_4`
  (params (Key :type "Key Structure"))
  (bind _sequenceplayer (`LevelSequenceActor.SequencePlayer` (`self.Sequence4`)))
  ;[1 1 1] Sequence 4 Control
  (:`Pressed`
    (if (`MovieSceneSequencePlayer.IsPlaying` _sequenceplayer)
      (`MovieSceneSequencePlayer.Pause` _sequenceplayer)
      (else
        (`MovieSceneSequencePlayer.Play` _sequenceplayer)))))

(event `InputAction|VP_Triggerable_4_Stop`
  (params (Key :type "Key Structure"))
  ;[1 1 1] Sequence 4 Control
  (:`Pressed`
    (`MovieSceneSequencePlayer.Stop` (`LevelSequenceActor.SequencePlayer` (`self.Sequence4`)))))

(event `InputAction|VP_Triggerable_Actor_1`
  (params (Key :type "Key Structure"))
  (bind (_actoraction1_actor _actoraction1_action) (break `/Game/VPToolKit/BluePrint/VPTK_ActorAction` (`self.ActorAction1`)))
  ;[1 1 1] Trigger Actors
  (:`Pressed`
    (bind _asvptk_itriggerable_actor (cast `/Game/VPToolKit/BluePrint/VPTK_ITriggerableActor` _actoraction1_actor))
    (`/Game/VPToolKit/BluePrint/VPTK_ITriggerableActor.TriggerAction` _asvptk_itriggerable_actor _actoraction1_action)))

(event `InputAction|VP_Triggerable_Actor_2`
  (params (Key :type "Key Structure"))
  (bind (_actoraction2_actor _actoraction2_action) (break `/Game/VPToolKit/BluePrint/VPTK_ActorAction` (`self.ActorAction2`)))
  ;[1 1 1] Trigger Actors
  (:`Pressed`
    (bind _asvptk_itriggerable_actor (cast `/Game/VPToolKit/BluePrint/VPTK_ITriggerableActor` _actoraction2_actor))
    (`/Game/VPToolKit/BluePrint/VPTK_ITriggerableActor.TriggerAction` _asvptk_itriggerable_actor _actoraction2_action)))

(event `InputAction|VP_Triggerable_Actor_3`
  (params (Key :type "Key Structure"))
  (bind (_actoraction3_actor _actoraction3_action) (break `/Game/VPToolKit/BluePrint/VPTK_ActorAction` (`self.ActorAction3`)))
  ;[1 1 1] Trigger Actors
  (:`Pressed`
    (bind _asvptk_itriggerable_actor (cast `/Game/VPToolKit/BluePrint/VPTK_ITriggerableActor` _actoraction3_actor))
    (`/Game/VPToolKit/BluePrint/VPTK_ITriggerableActor.TriggerAction` _asvptk_itriggerable_actor _actoraction3_action)))

(event `InputAction|VP_Triggerable_Actor_4`
  (params (Key :type "Key Structure"))
  (bind (_actoraction4_actor _actoraction4_action) (break `/Game/VPToolKit/BluePrint/VPTK_ActorAction` (`self.ActorAction4`)))
  ;[1 1 1] Trigger Actors
  (:`Pressed`
    (bind _asvptk_itriggerable_actor (cast `/Game/VPToolKit/BluePrint/VPTK_ITriggerableActor` _actoraction4_actor))
    (`/Game/VPToolKit/BluePrint/VPTK_ITriggerableActor.TriggerAction` _asvptk_itriggerable_actor _actoraction4_action)))

(fn `Assign Actor to Tracker`
  (params (TrackedActorName :type String) (TrackerID :type Integer))
  (returns (Success :type Boolean))
  (locals (ReturnValue :type Boolean) (localTrackerVirObjRef :type "Actor Object Reference") (localHeadObjRef :type "Actor Object Reference") (localActorCompRef :type "/Game/VPToolKit/BluePrint/VPTK_TrackedActorComponent Object Reference"))
  (bind _trackedentities (`self.TrackedEntities`))
  (bind (_value _returnvalue) (`BlueprintMapLibrary.Map_Find` _trackedentities TrackedActorName))
  ;[1 1 1] Try to assign to desired IDs
  (set `local.ReturnValue` false)
  (if _returnvalue
    ;;[1 1 1] Persist refs to objects because reasons
    (set `local.localTrackerVirObjRef` (`.TrackerVirtualObject_8_3B16C4C141F8D81EF7647BA531DB1EB0` (break `/Game/VPToolKit/BluePrint/VPTK_TrackedEntity` _value)))
    (set `local.localHeadObjRef` (`.TrackerHeadObject_10_E5988AD848B71EF4BF35CF813305BAA1` (break `/Game/VPToolKit/BluePrint/VPTK_TrackedEntity` _value)))
    (set `local.localActorCompRef` (`.TrackedActorComponent_14_D43A9CD84B528C7316EC1EBA682D77DA` (break `/Game/VPToolKit/BluePrint/VPTK_TrackedEntity` _value)))
    (for _array_element (`self.AvaliableTrackingIds`)
      (if (== _array_element TrackerID)
        (`/Game/VPToolKit/BluePrint/VPTK_TrackedActorComponent.AssignToTracker` (`.TrackedActorComponent_14_D43A9CD84B528C7316EC1EBA682D77DA` (break `/Game/VPToolKit/BluePrint/VPTK_TrackedEntity` _value)) TrackerID (`.TrackerHeadObject_10_E5988AD848B71EF4BF35CF813305BAA1` (break `/Game/VPToolKit/BluePrint/VPTK_TrackedEntity` _value)))
        ;;[1 1 1] Update the map with the new tracker ID
        (`BlueprintMapLibrary.Map_Remove` _trackedentities TrackedActorName)
        (`BlueprintMapLibrary.Map_Add` _trackedentities TrackedActorName (make `/Game/VPToolKit/BluePrint/VPTK_TrackedEntity` TrackerID (`local.localTrackerVirObjRef`) (`local.localHeadObjRef`) (`local.localActorCompRef`)))
        ;;[1 1 1] If the tracker is a Camera update the world view
        (set `local.ReturnValue` true)
        (if (`/Game/VPToolKit/BluePrint/VPTK_TrackedActorComponent.Is Camera` (`.TrackedActorComponent_14_D43A9CD84B528C7316EC1EBA682D77DA` (break `/Game/VPToolKit/BluePrint/VPTK_TrackedEntity` _value)))
          (`self.WriteVPLog` (`KismetStringLibrary.Concat_StrStr` "Trying to set active camera to TrackedActorComonent : " (`/Game/VPToolKit/BluePrint/VPTK_TrackedActorComponent.Name` (`.TrackedActorComponent_14_D43A9CD84B528C7316EC1EBA682D77DA` (break `/Game/VPToolKit/BluePrint/VPTK_TrackedEntity` _value)))))
          (`PlayerController.SetViewTargetWithBlend` (`GameplayStatics.GetPlayerController` 0) (`ActorComponent.GetOwner` (`.TrackedActorComponent_14_D43A9CD84B528C7316EC1EBA682D77DA` (break `/Game/VPToolKit/BluePrint/VPTK_TrackedEntity` _value))) 0.0 "VTBlend_Linear" 0.0 false))
        (return (`local.ReturnValue`))))
    (else
      ;;[1 0.147 0.1329] Error handling
      (`self.WriteVPLog` (`KismetStringLibrary.Concat_StrStr` "Invalid Tacked Actor name \"" TrackedActorName "\" passed to AssignActor call"))))
  (set `local.ReturnValue` false)
  (return (`local.ReturnValue`)))

(fn `Get Tracked Actor Current Tracker ID`
  (params (TrackedActorName :type String))
  (returns (trackerID :type Integer))
  (bind (_value _returnvalue) (`BlueprintMapLibrary.Map_Find` (`self.TrackedEntities`) TrackedActorName))
  (if _returnvalue
    (return (break `/Game/VPToolKit/BluePrint/VPTK_TrackedEntity` _value))
    (else
      (return -1))))

(fn `GetAvaliableTrackingIDs`
  (returns (trackingIDs :type "Array of Integer"))
  (return (`self.AvaliableTrackingIds`)))

(fn `GetTrackedActorComponent`
  (params (Actor :type "Actor Object Reference"))
  (returns (`Tracked Actor Component` :type "/Game/VPToolKit/BluePrint/VPTK_TrackedActorComponent Object Reference"))
  (bind _returnvalue (`self.K2_GetComponentsByClass` Actor "/Game/VPToolKit/BluePrint/VPTK_TrackedActorComponent.VPTK_TrackedActorComponent_C"))
  (if (== (`KismetArrayLibrary.Array_Length` _returnvalue) 1)
    (for _array_element _returnvalue
      (return _array_element))
    (else
      (`self.WriteVPLog` (`KismetStringLibrary.BuildString_Object` "" "VPTK Controller failed to fine VPTKTrackedActorComponent on : " Actor))
      (return null))))

(fn `GetTrackedActorNames`
  (returns (Names :type "Array of String"))
  (bind _keys (`BlueprintMapLibrary.Map_Keys` (`self.TrackedEntities`)))
  (return _keys))

(fn `UpdateActorAction`
  (params (slotID :type String) (NewAction :type String))
  (bind _actoraction1_actor (break `/Game/VPToolKit/BluePrint/VPTK_ActorAction` (`self.ActorAction1`)))
  (bind _actoraction3_actor (break `/Game/VPToolKit/BluePrint/VPTK_ActorAction` (`self.ActorAction3`)))
  (bind _actoraction2_actor (break `/Game/VPToolKit/BluePrint/VPTK_ActorAction` (`self.ActorAction2`)))
  (bind _actoraction4_actor (break `/Game/VPToolKit/BluePrint/VPTK_ActorAction` (`self.ActorAction4`)))
  ;[1 1 1] TODO: Everything about ActorActions is ugly....and I hate structs in UE Blueprints
  (switch `string` slotID
    (:`6`
      (set `self.ActorAction1` (make `/Game/VPToolKit/BluePrint/VPTK_ActorAction` _actoraction1_actor NewAction)))
    (:`7`
      (set `self.ActorAction2` (make `/Game/VPToolKit/BluePrint/VPTK_ActorAction` _actoraction2_actor NewAction)))
    (:`8`
      (set `self.ActorAction3` (make `/Game/VPToolKit/BluePrint/VPTK_ActorAction` _actoraction3_actor NewAction)))
    (:`9`
      (set `self.ActorAction4` (make `/Game/VPToolKit/BluePrint/VPTK_ActorAction` _actoraction4_actor NewAction)))))

(fn `UserConstructionScript`
  (locals (TrackingVolColor :type "LinearColor Structure" :default (struct :`R` 0.871367 :`G` 0.056128 :`B` 0.084376 :`A` 1.0)))
  (bind (_trackingvolumeextents_x _trackingvolumeextents_y _trackingvolumeextents_z) (`KismetMathLibrary.BreakVector` (`self.TrackingVolumeExtents`)))
  (bind _volumeoffset (`self.VolumeOffset`))
  (bind (_returnvalue_x _returnvalue_y _returnvalue_z) (`KismetMathLibrary.BreakVector` (`SceneComponent.K2_GetComponentLocation` _volumeoffset)))
  (if (`self.DisplayDebugVolume`)
    (`KismetSystemLibrary.FlushPersistentDebugLines`)
    (`KismetSystemLibrary.DrawDebugBox` (`KismetMathLibrary.MakeVector` _returnvalue_x _returnvalue_y (+ _returnvalue_z _trackingvolumeextents_z)) (`self.TrackingVolumeExtents`) (`local.TrackingVolColor`) (`SceneComponent.K2_GetComponentRotation` _volumeoffset) 120.0 2.0)))